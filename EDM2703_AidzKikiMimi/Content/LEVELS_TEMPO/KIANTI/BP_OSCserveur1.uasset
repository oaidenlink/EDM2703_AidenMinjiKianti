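; BP_OSCserveur1 is an OSC receiver that relays incoming Open Sound Control messages to actors in the level.
; On BeginPlay it starts an OSC server listening on port 10000 on all addresses and caches every actor implementing BPI_OSCInterface.
; Each received message passes its full address path as ID and its first float as Value to those cached actors through the interface.
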(event `self.ReceiveBeginPlay`
  (bind _returnvalue (`OSCManager.CreateOSCServer` "0.0.0.0" 10000 false true "" null))
  (bind _output_get (set `self.OSC_Server` _returnvalue))
  (add `OSCServer.OnOscMessageReceived` _output_get (delegate `OSCmsg`))
  (bind _outactors (`GameplayStatics.GetAllActorsWithInterface` "/Game/LEVELS_TEMPO/KIANTI/BPI_OSCInterface.BPI_OSCInterface_C"))
  (bind _output_get_2 (set `self.OSCInterfaceActors` _outactors)))

(event `OSCmsg`
  (params (Message :type "OSCMessage Structure (by ref)") (IPAddress :type String) (Port :type Integer))
  (bind _returnvalue (`OSCManager.GetOSCMessageAddress` Message))
  (bind _returnvalue_2 (`OSCManager.GetOSCAddressFullPath` _returnvalue))
  (bind _value (`OSCManager.GetFloat` Message))
  (message `/Game/LEVELS_TEMPO/KIANTI/BPI_OSCInterface.OSCMessage` (stale `self.ReceiveBeginPlay` _output_get_2) _returnvalue_2 _value))

(fn `UserConstructionScript`)