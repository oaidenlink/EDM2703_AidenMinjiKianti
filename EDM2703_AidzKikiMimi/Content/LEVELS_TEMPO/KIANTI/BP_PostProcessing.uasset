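; BP_PostProcessing lets MIDI input on channel 3 drive level visuals live.
; Control 77 maps to exposure compensation, with a dead zone snapping near-center values to zero, written to the PostProcessVolume found in the level.
; Note 40 switches the Glitch scalar in the MCP_Box parameter collection on or off by its value.
; BeginPlay also creates a dynamic M_Tree1Emissive material instance, which is stored but otherwise unused here.
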(event `/Game/LEVELS_TEMPO/KIANTI/BPI_MIDIInterface.MIDIControl`
  (params (Channel :type Integer) (ID :type Integer) (Value :type Integer))
  (bind _returnvalue (`KismetMathLibrary.MapRangeClamped` (`KismetMathLibrary.Conv_IntToDouble` Value) 0.0 127.0 -5.0 5.0))
  (if (== Channel 3)
    (switch `int` ID
      (:`77`
        (bind _output_get (set `self.Exposure` (`KismetMathLibrary.SelectFloat` 0.0 _returnvalue (< (`KismetMathLibrary.Abs` _returnvalue) 0.2))))
        (bind _returnvalue_2 (`GameplayStatics.GetActorOfClass` "/Script/Engine.PostProcessVolume"))
        (setmembers `PostProcessSettings` :`StructRef` (`PostProcessVolume.Settings` _returnvalue_2) :`AutoExposureBias` _output_get)))))

(event `/Game/LEVELS_TEMPO/KIANTI/BPI_MIDIInterface.MIDINote`
  (params (Channel :type Integer) (ID :type Integer) (Value :type Integer))
  (if (== Channel 3)
    (switch `int` ID
      (:`40`
        (bind _output_get (set `self.Glitch` (`KismetMathLibrary.SelectFloat` 0.0 1.0 (< (`KismetMathLibrary.Conv_IntToDouble` Value) 0.2))))
        (`KismetMaterialLibrary.SetScalarParameterValue` "/Game/LEVELS_TEMPO/KIANTI/MCP_Box.MCP_Box" "Glitch" _output_get)
        (`KismetSystemLibrary.PrintString` (`KismetStringLibrary.Conv_DoubleToString` _output_get))))))

(event `self.ReceiveBeginPlay`
  (bind _returnvalue (`KismetMaterialLibrary.CreateDynamicMaterialInstance` "/Game/LEVELS_TEMPO/KIANTI/ForestAssets/Materials/M_Tree1Emissive.M_Tree1Emissive" "Glitch"))
  (set `self.TreeDynMat` _returnvalue))

(fn `UserConstructionScript`)