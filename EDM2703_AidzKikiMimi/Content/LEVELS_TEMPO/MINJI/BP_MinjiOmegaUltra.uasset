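; BP_MinjiOmegaUltra is a trigger actor that changes light and sound when the first-person character enters its AAAcollision volume.
; On overlap it turns the SpotLight cyan, plays AmbianceSombre at the actor's location with a loud volume multiplier and attenuation, and stops the MSAudioTest1 audio.
; When any overlap ends it turns the light red, without checking the actor or restoring the audio.
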(event `self.AAAcollision.OnComponentBeginOverlap`
  (params (OverlappedComponent :type "PrimitiveComponent Object Reference") (OtherActor :type "Actor Object Reference") (OtherComp :type "PrimitiveComponent Object Reference") (OtherBodyIndex :type Integer) (bFromSweep :type Boolean) (SweepResult :type "HitResult Structure (by ref)"))
  (cast `/Game/FirstPerson/Blueprints/BP_FirstPersonCharacter` OtherActor)
  (`LightComponent.SetLightColor` (`self.SpotLight`) (struct :`R` 0.012286 :`G` 1.0 :`B` 0.896269 :`A` 1.0) true)
  (`GameplayStatics.PlaySoundAtLocation` "/Game/LEVELS_TEMPO/MINJI/Audio/AmbianceSombre.AmbianceSombre" (`self.K2_GetActorLocation` (`ActorComponent.GetOwner` (`self.AAAcollision`))) (struct) 50.0 1.0 0.0 "/Game/LEVELS_TEMPO/MINJI/A_TriggerMinji.A_TriggerMinji" null null null)
  (`AudioComponent.Stop` (`self.MS_audioTest1`)))

(event `self.AAAcollision.OnComponentEndOverlap`
  (params (OverlappedComponent :type "PrimitiveComponent Object Reference") (OtherActor :type "Actor Object Reference") (OtherComp :type "PrimitiveComponent Object Reference") (OtherBodyIndex :type Integer))
  (`LightComponent.SetLightColor` (`self.SpotLight`) (struct :`R` 0.733333 :`A` 1.0) true))

(fn `UserConstructionScript`)