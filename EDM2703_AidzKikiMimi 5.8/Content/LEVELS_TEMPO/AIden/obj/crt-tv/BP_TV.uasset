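; BP_TV is a scare trigger that fires when BP_FirstPersonCharacter overlaps its box.
; The overlap brightens a spotlight, fades in scary audio, adds two audio components and plays the Pos_Main timeline to animate BPHand.
; Each Pos_Main update switches off five orange lights and calls Play on LumBleu, which drives four blue lights.
; LumBleu's update also runs a short delay that fades the scary audio out.
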(event `self.Box.OnComponentBeginOverlap`
  (params (OverlappedComponent :type "PrimitiveComponent Object Reference") (OtherActor :type "Actor Object Reference") (OtherComp :type "PrimitiveComponent Object Reference") (OtherBodyIndex :type Integer) (bFromSweep :type Boolean) (SweepResult :type "HitResult Structure (by ref)"))
  (cast `/Game/FirstPerson/Blueprints/BP_FirstPersonCharacter` OtherActor)
  (`LightComponent.SetIntensity` (`self.SpotLight`) 8.0)
  (`AudioComponent.FadeIn` (`self.MS_ScaryAudioOOH`) 1.0 1.0 0.0 "Linear")
  (`AddComponent|NODE_AddAudioComponent-5`)
  (`AddComponent|NODE_AddAudioComponent-4`)
  (bind (_direction _posy _posz _rotx) (`Timeline|pos_Main`)
    (:`Update`
      (`SceneComponent.K2_SetRelativeLocationAndRotation` (`self.BP_Hand`) (`KismetMathLibrary.MakeVector` 0.0 (* _posy 80.0) _posz) (`KismetMathLibrary.MakeRotator` _rotx) false false)
      (`LightComponent.SetIntensity` (`self.Orange1`) 0.0)
      (`LightComponent.SetIntensity` (`self.Orange2`) 0.0)
      (`LightComponent.SetIntensity` (`self.Orange3`) 0.0)
      (`LightComponent.SetIntensity` (`self.Orange4`) 0.0)
      (`LightComponent.SetIntensity` (`self.Orange5`) 0.0)
      (bind (_direction_2 _light1 _light2 _light3 _light4) (`Timeline|lumBleu`)
        (:`Update`
          (`LightComponent.SetIntensity` (`self.BlueLight1`) _light1)
          (`LightComponent.SetIntensity` (`self.BlueLight2`) _light2)
          (`LightComponent.SetIntensity` (`self.BlueLight3`) _light3)
          (`LightComponent.SetIntensity` (`self.BlueLight4`) _light4)
          (`KismetSystemLibrary.Delay` 1.0)
          (`AudioComponent.FadeOut` (`self.MS_ScaryAudioOOH`) 2.0 0.0 "Linear"))))))

(fn `UserConstructionScript`)